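; BP_Key is a key pickup that the player collects by pressing E, provided their Money is at least 4000.
; Success passes the item to the player's GrabItem, plays a sound, sets the game mode's Key flag and destroys the actor; otherwise ShowText displays a message.
; The E check uses the box's overlapping actor.
; Both begin and end overlap call EnableInput, so input is never disabled on exit.
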(event OnComponentBeginOverlap(Box)
  (params (OverlappedComponent :type Primitive%20Component%20Object%20Reference) (OtherActor :type Actor%20Object%20Reference) (OtherComp :type Primitive%20Component%20Object%20Reference) (OtherBodyIndex :type Integer) (bFromSweep :type Boolean) (SweepResult :type Hit%20Result%20Structure%20%28by%20ref%29))
  (Input|EnableInput (Game|GetPlayerController 0)))

(event OnComponentEndOverlap(Box)
  (params (OverlappedComponent :type Primitive%20Component%20Object%20Reference) (OtherActor :type Actor%20Object%20Reference) (OtherComp :type Primitive%20Component%20Object%20Reference) (OtherBodyIndex :type Integer))
  (Input|EnableInput (Game|GetPlayerController 0)))

(event Input|KeyboardEvents|E
  (params (Key :type Key%20Structure))
  (:Pressed
    (bind _asbp_third_person_character (Utilities|Casting|CastToBP_ThirdPersonCharacter (stale OnComponentBeginOverlap(Box) OtherActor)))
    (if (>= (Variables|/Game/ThirdPerson/Blueprints/BP_ThirdPersonCharacter.BP_ThirdPersonCharacter_C|GetMoney _asbp_third_person_character) 4e+03)
      (bind _asbp_third_person_game_mode (Utilities|Casting|CastToBP_ThirdPersonGameMode (Game|GetGameMode)))
      (bind _asbp_third_person_character_2 (Utilities|Casting|CastToBP_ThirdPersonCharacter (Game|GetPlayerCharacter 0)))
      (Default|GrabItem _asbp_third_person_character_2 (Variables|Default|Getitem))
      (Audio|PlaySound2D "/Game/multimedia/Sounds/agarrarLlave.agarrarLlave" 1.0 1.0 0.0 0 0)
      (Variables|/Game/ThirdPerson/Blueprints/BP_ThirdPersonGameMode.BP_ThirdPersonGameMode_C|Setkey? _asbp_third_person_game_mode true)
      (Actor|DestroyActor)
      (else
        (Default|ShowText _asbp_third_person_character 5)))))

(fn ConstructionScript)