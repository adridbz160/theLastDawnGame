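; BP_MoneyBag is a consumable money pickup that gives the third-person player character a random amount of money up to 1000.
; On box overlap with that character, it adds the money, prints the new total, plays the pickup sound and destroys itself.
; The pre-pickup balance selects one of three duplicated branches: zero or less calls ShowText(1), 4000 or more calls ShowText(2), and anything between shows no text.
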(event OnComponentBeginOverlap(Box)
  (params (OverlappedComponent :type Primitive%20Component%20Object%20Reference) (OtherActor :type Actor%20Object%20Reference) (OtherComp :type Primitive%20Component%20Object%20Reference) (OtherBodyIndex :type Integer) (bFromSweep :type Boolean) (SweepResult :type Hit%20Result%20Structure%20%28by%20ref%29))
  ;[1 1 1] Moneda Consumible
  (bind _asbp_third_person_character (Utilities|Casting|CastToBP_ThirdPersonCharacter OtherActor))
  (if (<= (Variables|/Game/ThirdPerson/Blueprints/BP_ThirdPersonCharacter.BP_ThirdPersonCharacter_C|GetMoney _asbp_third_person_character) 0)
    (bind _output_get (Variables|/Game/ThirdPerson/Blueprints/BP_ThirdPersonCharacter.BP_ThirdPersonCharacter_C|SetMoney _asbp_third_person_character (+ (Variables|/Game/ThirdPerson/Blueprints/BP_ThirdPersonCharacter.BP_ThirdPersonCharacter_C|GetMoney _asbp_third_person_character) (Math|Random|RandomIntegerinRange 0 1000))))
    (Development|PrintString (Utilities|String|ToString(Integer) _output_get))
    (Audio|PlaySound2D "/Game/multimedia/Sounds/itemGet.itemGet" 1.0 1.0 0.0 0 0)
    (Actor|DestroyActor)
    (Default|ShowText _asbp_third_person_character 1)
    (elif (>= (Variables|/Game/ThirdPerson/Blueprints/BP_ThirdPersonCharacter.BP_ThirdPersonCharacter_C|GetMoney _asbp_third_person_character) 4000)
      (bind _output_get_2 (Variables|/Game/ThirdPerson/Blueprints/BP_ThirdPersonCharacter.BP_ThirdPersonCharacter_C|SetMoney _asbp_third_person_character (+ (Variables|/Game/ThirdPerson/Blueprints/BP_ThirdPersonCharacter.BP_ThirdPersonCharacter_C|GetMoney _asbp_third_person_character) (Math|Random|RandomIntegerinRange 0 1000))))
      (Development|PrintString (Utilities|String|ToString(Integer) _output_get_2))
      (Audio|PlaySound2D "/Game/multimedia/Sounds/itemGet.itemGet" 1.0 1.0 0.0 0 0)
      (Actor|DestroyActor)
      (Default|ShowText _asbp_third_person_character 2)
      (else
        (bind _output_get_3 (Variables|/Game/ThirdPerson/Blueprints/BP_ThirdPersonCharacter.BP_ThirdPersonCharacter_C|SetMoney _asbp_third_person_character (+ (Variables|/Game/ThirdPerson/Blueprints/BP_ThirdPersonCharacter.BP_ThirdPersonCharacter_C|GetMoney _asbp_third_person_character) (Math|Random|RandomIntegerinRange 0 1000))))
        (Development|PrintString (Utilities|String|ToString(Integer) _output_get_3))
        (Audio|PlaySound2D "/Game/multimedia/Sounds/itemGet.itemGet" 1.0 1.0 0.0 0 0)
        (Actor|DestroyActor)))))

(fn ConstructionScript)