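; BP_Smoke is a level decoration hazard that hurts the player while they are inside its sphere.
; When a BP_ThirdPersonCharacter enters, it sets a flag and applies random damage to player 0 in a Delay-driven loop.
; The loop repeats until the flag clears or that character's PlayerHealth reaches zero.
; Any actor leaving the sphere clears the flag, as end overlap has no actor check.
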(event OnComponentBeginOverlap(Sphere)
  (params (OverlappedComponent :type Primitive%20Component%20Object%20Reference) (OtherActor :type Actor%20Object%20Reference) (OtherComp :type Primitive%20Component%20Object%20Reference) (OtherBodyIndex :type Integer) (bFromSweep :type Boolean) (SweepResult :type Hit%20Result%20Structure%20%28by%20ref%29))
  (bind _asbp_third_person_character (Utilities|Casting|CastToBP_ThirdPersonCharacter OtherActor))
  (Variables|Default|Setdaño? true)
  (Game|Damage|ApplyDamage (Game|GetPlayerCharacter 0) (Math|Random|RandomFloatinRange 5.0 2e+01) 0 0 :!label _label)
  (Utilities|FlowControl|Delay 0.6)
  (if (Variables|Default|Getdaño?)
    (if (not (<= (Variables|/Game/ThirdPerson/Blueprints/BP_ThirdPersonCharacter.BP_ThirdPersonCharacter_C|GetplayerHealth _asbp_third_person_character) 0.0))
      (goto _label))))

(event OnComponentEndOverlap(Sphere)
  (params (OverlappedComponent :type Primitive%20Component%20Object%20Reference) (OtherActor :type Actor%20Object%20Reference) (OtherComp :type Primitive%20Component%20Object%20Reference) (OtherBodyIndex :type Integer))
  (Variables|Default|Setdaño? false))

(fn ConstructionScript)