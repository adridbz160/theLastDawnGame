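; BP_Bed is an interactable bed that ends the current level and loads the BG_StartHUD level.
; Its Box overlap events enable and disable the actor's input for player controller 0, without checking which actor overlaps.
; Pressing E while input is enabled plays a bird sound and shows the WB_FinishScreenHUD widget.
; After a short delay, it removes the widget and opens the level.
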(event OnComponentBeginOverlap(Box)
  (params (OverlappedComponent :type Primitive%20Component%20Object%20Reference) (OtherActor :type Actor%20Object%20Reference) (OtherComp :type Primitive%20Component%20Object%20Reference) (OtherBodyIndex :type Integer) (bFromSweep :type Boolean) (SweepResult :type Hit%20Result%20Structure%20%28by%20ref%29))
  (Input|EnableInput (Game|GetPlayerController 0)))

(event OnComponentEndOverlap(Box)
  (params (OverlappedComponent :type Primitive%20Component%20Object%20Reference) (OtherActor :type Actor%20Object%20Reference) (OtherComp :type Primitive%20Component%20Object%20Reference) (OtherBodyIndex :type Integer))
  (Input|DisableInput (Game|GetPlayerController 0)))

(event Input|KeyboardEvents|E
  (params (Key :type Key%20Structure))
  (:Pressed
    (Audio|PlaySound2D "/Game/StarterContent/Audio/Starter_Birds01.Starter_Birds01" 1.0 1.0 0.0 0 0)
    (bind _returnvalue (UserInterface|CreateWidget "/Game/HUDs/FinishScreen/WB_FinishScreenHUD.WB_FinishScreenHUD_C"))
    (UserInterface|Viewport|AddtoViewport _returnvalue 0)
    (Utilities|FlowControl|Delay 5.0)
    (Widget|RemovefromParent _returnvalue)
    (Game|OpenLevel(byObjectReference) "/Game/HUDs/StartHUD/BG_StartHUD.BG_StartHUD")))

(fn ConstructionScript)